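; BP_Flower is a flower actor whose color follows a numerical simulation run by GM_FlowerSim.
; BeginPlay creates a dynamic instance of MI_Flower on the flower mesh.
; Each tick, it maps its world position to clamped grid indices using hardcoded area bounds and the simulation's DiscretizationN.
; It then reads that cell from the game mode's flattened color array and writes it to a scalar material parameter.
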(event `self.ReceiveBeginPlay`
  ;[1 0.9489 0.3335] This is to set a material instance so that can change color according to the simulation
  (bind _returnvalue (`PrimitiveComponent.CreateDynamicMaterialInstance` (`self.SMBP_Flower`) 0 "/Game/FlowerImport/MI_Flower.MI_Flower" "None"))
  (set `self.MaterialInstance` _returnvalue))

(event `self.ReceiveTick`
  (params (DeltaSeconds :type "Float (single-precision)"))
  ;[0.3641 1 0.9068] This is to change, at each tick, the color of the flower according to the value of the simulation
  (cast `/Game/GM_FlowerSim` (`GameplayStatics.GetGameMode`))
  (bind _asgm_flower_sim (cast `/Game/GM_FlowerSim` (`GameplayStatics.GetGameMode`)))
  (bind (_x _y) (`self.ObtainPositionsXYindex`))
  (`MaterialInstanceDynamic.SetScalarParameterValue` (`self.MaterialInstance`) "ValueColorParameterMaterial" (`|GetArrayItem` (`/Game/GM_FlowerSim.ColorMatrixesInArrayFormat` _asgm_flower_sim) (+ _x (* _y (`/Game/GM_FlowerSim.DiscretizationN` _asgm_flower_sim))))))

(fn `ObtainPositionsXYindex`
  (returns (X :type Integer) (Y :type Integer))
  (bind (_returnvalue_x _returnvalue_y) (`KismetMathLibrary.BreakVector` (`SceneComponent.K2_GetComponentLocation` (`self.DefaultSceneRoot`))))
  ;[1 1 1] This functions uses the position of the flower in the space (in world coordinates) to return indexes (X,Y) corresponding to the position in the grid of the numerical simulation
  (bind _asgm_flower_sim (cast `/Game/GM_FlowerSim` (`GameplayStatics.GetGameMode`)))
  (bind _returnvalue (- (`/Game/GM_FlowerSim.DiscretizationN` _asgm_flower_sim) 1))
  (bind _returnvalue_2 (`KismetMathLibrary.Conv_IntToDouble` _returnvalue))
  (return (`KismetMathLibrary.Min` (`KismetMathLibrary.Max` (`KismetMathLibrary.FTrunc` (* (/ (- _returnvalue_x 910.0) -2830.0) _returnvalue_2))) _returnvalue) (`KismetMathLibrary.Min` _returnvalue (`KismetMathLibrary.Max` (`KismetMathLibrary.FTrunc` (* (/ (- _returnvalue_y 420.0) -1520.0) _returnvalue_2))))))

(fn `UserConstructionScript`)