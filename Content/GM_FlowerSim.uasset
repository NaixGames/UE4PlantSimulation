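; GM_FlowerSim runs a 2D Allen-Cahn-style reaction-diffusion simulation on an NxN grid stored as a flattened float array.
; BeginPlay computes the diffusion coefficient and seeds the grid with a cross shape; square and Batman-like seeds exist but are unconnected.
; After the start input, each Tick with time left takes an explicit Euler step from a copied grid, combining a cubic reaction term with a five-point Laplacian using modulo-indexed neighbours.
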(event `self.ReceiveBeginPlay`
  (bind _discretizationn (`self.DiscretizationN`))
  (bind _discretizationn_2 (`self.DiscretizationN`))
  ;[1 0.2604 0.826] This is to recieve inputs and set some useful parameters
  (`self.EnableInput` (`GameplayStatics.GetPlayerController` 0))
  (bind _output_get (set `self.DeltaXSq` (`KismetMathLibrary.Square` (/ 2.0 (`KismetMathLibrary.Conv_IntToDouble` (`self.DiscretizationN`))))))
  (set `self.Coecientdtdx` (/ (`self.DeltaTime`) _output_get))
  ;[1 0.2778 0.2778] At the start we set some color matrix for a initial condition
  ;;[1 1 1] This part resize the array for an NxN grid
  (`KismetArrayLibrary.Array_Resize` (`self.ColorMatrixesInArrayFormat`) (* _discretizationn _discretizationn))
  ;;[1 1 1] We assing each element in the array the corresponding value for a initial condition. For different simulations change X Initial Condition to another function as the one above
  (for (_ _array_index) (`self.ColorMatrixesInArrayFormat`)
    (bind _outputvalue (`self.CrossInitialCondition` (/ _array_index _discretizationn_2) (mod _array_index _discretizationn_2)))
    (`KismetArrayLibrary.Array_Set` (`self.ColorMatrixesInArrayFormat`) _array_index _outputvalue))
  (`KismetSystemLibrary.PrintString` "Simulation ready, press Z or P to begin"))

(event `InputAction|StartSimulationButton`
  (params (Key :type "Key Structure"))
  ;[0.4479 0.9889 1] Only start simualtion after pressing play
  (:`Pressed`
    (set `self.PlayVariable` true)))

(event `self.ReceiveTick`
  (params (DeltaSeconds :type "Float (single-precision)"))
  (bind _discretizationn (`self.DiscretizationN`))
  (bind _discretizationn_2 (`self.DiscretizationN`))
  (bind _colormatrixesinarrayformat (`self.ColorMatrixesInArrayFormat`))
  ;[1 0.9521 0.1756] We make sure the run the simulation for the required time after we press play
  (if (and (`self.PlayVariable`) (`self.IsTimeLeft`))
    ;[0.0842 1 0.8736] In this bit we compute a temporal step in the simulation. Do not modify this bit!
    (set `self.OldTimeMatrix` _colormatrixesinarrayformat)
    (for (_ _array_index) _colormatrixesinarrayformat
      (bind _output (`|GetArrayItem` (`self.OldTimeMatrix`) _array_index))
      (bind _result (`self.ACNonlinear Term` _output))
      (bind _output_get (set `self.ComputationVariable` (+ _result (* _output (- 1.0 (* 4.0 (`self.Coecientdtdx`)))))))
      (bind _returnvalue (/ _array_index _discretizationn))
      (bind _returnvalue_2 (mod _array_index _discretizationn))
      (bind _returnvalue_3 (* _returnvalue (`self.DiscretizationN`)))
      (bind _output_get_2 (set `self.ComputationVariable` (+ _output_get (* (+ (`|GetArrayItem` (`self.OldTimeMatrix`) (+ (* (mod (+ _returnvalue 1) _discretizationn) _discretizationn_2) _returnvalue_2)) (`|GetArrayItem` (`self.OldTimeMatrix`) (+ (* (mod (- _returnvalue 1) _discretizationn) _discretizationn_2) _returnvalue_2)) (`|GetArrayItem` (`self.OldTimeMatrix`) (+ (mod (+ _returnvalue_2 1) _discretizationn) _returnvalue_3)) (`|GetArrayItem` (`self.OldTimeMatrix`) (+ (mod (- _returnvalue_2 1) _discretizationn) _returnvalue_3))) (`self.Coecientdtdx`)))))
      (`KismetArrayLibrary.Array_Set` (`self.ColorMatrixesInArrayFormat`) _array_index _output_get_2))))

(fn `ACNonlinear Term`
  (params (Input :type "Float (double-precision)"))
  (returns (Result :type "Float (double-precision)"))
  ;[1 1 1] This function computes the non-linearity of the equation; \epsilon^{-2} u(1-u)(2u-(1-\epsilon \nu))
  (return (/ (* Input (- 1.0 Input) (- (* Input 2.0) (- 1.0 (* (`self.EpsilonVariable`) (`self.NuVariable`)))) (`self.DeltaTime`)) (`KismetMathLibrary.Square` (`self.EpsilonVariable`)))))

(fn `BatmanLikeInitialCondition`
  (params (Yaxis :type Integer) (Xaxis :type Integer))
  (returns (OutputValue :type "Float (double-precision)"))
  (bind _discretizationn (`self.DiscretizationN`))
  (bind _discretizationn_2 (`self.DiscretizationN`))
  (bind _discretizationn_3 (`self.DiscretizationN`))
  (bind _returnvalue (/ (`self.DiscretizationN`) 2))
  (bind _returnvalue_2 (`KismetMathLibrary.Abs_Int` (- Xaxis _returnvalue)))
  (bind _returnvalue_3 (`KismetMathLibrary.Abs_Int` (* (- Yaxis _returnvalue) -1)))
  ;[1 1 1] This function gives 1 if the index in the grid is in a batman symbol like shape arround the origin and 0 otherwise. Note; the batman symbol is not that good :(
  (if (and (>= (/ _discretizationn_2 12) _returnvalue_3) (>= (/ _discretizationn_2 4) _returnvalue_2))
    (return 1.0)
    (elif (and (>= (/ _discretizationn_3 4) _returnvalue_3) (>= (/ _discretizationn_3 10) _returnvalue_2))
      (return 1.0)
      (elif (and (>= (/ _discretizationn 5) _returnvalue_3) (>= _returnvalue_2 (/ _discretizationn 4)) (>= (/ _discretizationn 3) _returnvalue_2))
        (return 1.0)
        (else
          (return 0.0))))))

(fn `CrossInitialCondition`
  (params (Yaxis :type Integer) (Xaxis :type Integer))
  (returns (OutputValue :type "Float (double-precision)"))
  (bind _discretizationn (`self.DiscretizationN`))
  (bind _discretizationn_2 (`self.DiscretizationN`))
  (bind _returnvalue (/ (`self.DiscretizationN`) 2))
  (bind _returnvalue_2 (`KismetMathLibrary.Abs_Int` (- Xaxis _returnvalue)))
  (bind _returnvalue_3 (`KismetMathLibrary.Abs_Int` (* (- Yaxis _returnvalue) -1)))
  ;[1 1 1] This function gives 1 if the index in the grid is in a cross shape arround the origin and 0 otherwise
  (if (and (>= (/ _discretizationn_2 10) _returnvalue_3) (>= (/ _discretizationn_2 3) _returnvalue_2))
    (return 1.0)
    (elif (and (>= (/ _discretizationn 3) _returnvalue_3) (>= (/ _discretizationn 10) _returnvalue_2))
      (return 1.0)
      (else
        (return 0.0)))))

(fn `SquareInitialCondition`
  (params (Yaxis :type Integer) (Xaxis :type Integer))
  (returns (Value :type "Float (double-precision)"))
  (bind _returnvalue (/ (`self.DiscretizationN`) 4))
  (bind _returnvalue_2 (/ (`self.DiscretizationN`) 2))
  ;[1 1 1] This function gives 1 if the index in the grid is in a cube arround the origin and 0 otherwise
  (return (`KismetMathLibrary.Conv_BoolToDouble` (and (> _returnvalue (`KismetMathLibrary.Abs_Int` (* (- Yaxis _returnvalue_2) -1))) (> _returnvalue (`KismetMathLibrary.Abs_Int` (- Xaxis _returnvalue_2)))))))

(fn `UserConstructionScript`)